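; Golem actor that wakes when a BP_Vehicle rams it, shoving the vehicle with an impulse on every hit.
; The first hit sets IsRise and spawns a BP_GolemBullet attached to the right-hand projectile socket.
; After a five-second delay the crystal detaches, turns on physics and gains velocity toward the component that hit the golem.
; The looping timer for repeat shots is unwired, so it fires only once.
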(event OnComponentHit(SK_Golem_new)
  (params (HitComponent :type Primitive%20Component%20Object%20Reference) (OtherActor :type Actor%20Object%20Reference) (OtherComp :type Primitive%20Component%20Object%20Reference) (NormalImpulse :type Vector :default "0, 0, 0") (Hit :type Hit%20Result%20Structure%20%28by%20ref%29))
  (if (Utilities|ClassIsChildOf (Utilities|GetClass OtherActor) "/Game/Assets/Vehicule/BP_Vehicle.BP_Vehicle_C")
    (Physics|AddImpulse OtherComp (+ (* NormalImpulse "-1.000000,-1.000000,0.000000") "100.000000,100.000000,0.000000") "None" false)
    (Utilities|FlowControl|DoOnce false
      (:Completed
        (CallFunction|Rise)))))

(event Custom|CustomEvent
  (bind _returnvalue (Game|SpawnActorfromClass "/Game/Golem/BP_GolemBullet.BP_GolemBullet_C" (Math|Transform|MakeTransform (Transformation|GetWorldLocation (Variables|Default|GetBullet%20Spawn)) "0, 0, 0" "1.000000,1.000000,1.000000") "Undefined" "MultiplyWithRoot" 0 0))
  (Transformation|AttachComponentToComponent _returnvalue (Variables|Default|GetSK_Golem_new) "hand_r_projectile" "SnapToTarget" "KeepRelative" "KeepRelative" true)
  (Utilities|FlowControl|Delay 5.0)
  (Transformation|DetachFromActor _returnvalue "KeepWorld" "KeepWorld" "KeepWorld")
  (Physics|SetSimulatePhysics (Variables|/Game/Golem/BP_GolemBullet.BP_GolemBullet_C|Getcrystal_shot _returnvalue) true)
  (Physics|SetPhysicsLinearVelocity (Variables|/Game/Golem/BP_GolemBullet.BP_GolemBullet_C|Getcrystal_shot _returnvalue) (Math|Rotator|GetRotationXVector (Math|Rotator|FindLookatRotation (Transformation|GetActorLocation _returnvalue) (Transformation|GetWorldLocation (stale OnComponentHit(SK_Golem_new) OtherComp)))) true "None"))

(event Custom|Rise
  (Variables|Default|SetisRise true)
  (CallFunction|CustomEvent))

(event EventBeginPlay)

(fn ConstructionScript
  (Transformation|AttachComponentToComponent (Variables|Default|GetBullet%20Spawn) (Variables|Default|GetSK_Golem_new) "hand_r_projectile" "SnapToTarget" "SnapToTarget" "SnapToTarget" true))