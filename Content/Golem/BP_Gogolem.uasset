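; Golem enemy that wakes when a BP_Vehicle hits it, knocks the vehicle back and hurls crystal projectiles at it.
; Once risen, a looping timer randomly picks a hand, attaches a spawned BP_GolemBullet to its socket and sets an attack flag.
; Drop releases the bullet toward the vehicle.
; Other non-bullet hits drain Health; death swaps the skeletal mesh for a physics-driven geometry collection and destroys all bullets.
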(event OnComponentHit(SK_Golem_new)
  (params (HitComponent :type Primitive%20Component%20Object%20Reference) (OtherActor :type Actor%20Object%20Reference) (OtherComp :type Primitive%20Component%20Object%20Reference) (NormalImpulse :type Vector :default "0, 0, 0") (Hit :type Hit%20Result%20Structure%20%28by%20ref%29))
  (bind _returnvalue (Utilities|GetClass OtherActor))
  (bind _gc_golemdeath (Variables|Default|GetGC_GolemDeath))
  (if (Utilities|ClassIsChildOf _returnvalue "/Game/Assets/Vehicule/BP_Vehicle.BP_Vehicle_C")
    (bind _output_get (Variables|Default|SetVehicle OtherComp))
    (Physics|AddImpulse _output_get (+ (* NormalImpulse "-1.000000,-1.000000,0.000000") "100.000000,100.000000,0.000000") "None" false)
    (Utilities|FlowControl|DoOnce false
      (:Completed
        (CallFunction|Rise)))
    (elif (and (not (Utilities|ClassIsChildOf _returnvalue "/Game/Golem/BP_GolemBullet.BP_GolemBullet_C")) (Variables|Default|GetisRise))
      (bind _output_get_2 (Variables|Default|SetHealth (- (Variables|Default|GetHealth) 10)))
      (Development|PrintString (Utilities|String|ToString(Integer) (- (Variables|Default|GetHealth) 10)))
      (if (<= _output_get_2 0)
        (Variables|Default|SetisDeath true)
        (Utilities|FlowControl|Delay 1.5)
        (Rendering|SetVisibility _gc_golemdeath true false)
        (Physics|SetSimulatePhysics _gc_golemdeath true)
        (Components|DestroyComponent (Variables|Default|GetSK_Golem_new))
        (Physics|AddImpulse (Variables|Default|GetGC_GolemDeath) "0.000000,0.000000,-1000.000000" "None" true)
        (bind _outactors (Actor|GetAllActorsOfClass "/Game/Golem/BP_GolemBullet.BP_GolemBullet_C"))
        (for _array_element _outactors
          (Actor|DestroyActor _array_element))))))

(event Custom|AttackRight
  (bind _returnvalue (Game|SpawnActorfromClass "/Game/Golem/BP_GolemBullet.BP_GolemBullet_C" (Math|Transform|MakeTransform (Transformation|GetWorldLocation (Variables|Default|GetRight%20Bullet%20Spawn)) "0, 0, 0" "1.000000,1.000000,1.000000") "Undefined" "MultiplyWithRoot" 0 0))
  (bind _output_get (Variables|Default|SetCurrentBullet _returnvalue))
  (Transformation|AttachComponentToComponent _output_get (Variables|Default|GetSK_Golem_new) "hand_r_projectile" "SnapToTarget" "KeepRelative" "KeepRelative" true)
  (Utilities|FlowControl|Delay 2.0)
  (Variables|Default|SetisAttackRight true))

(event Custom|Rise
  (Variables|Default|SetisRise true)
  (Utilities|Time|SetTimerbyEvent (delegate Custom|Attack) 5.0 true))

(event Custom|Attack
  (Utilities|FlowControl|MultiGate true true -1
    (:Out%200
      (CallFunction|AttackRight))
    (:Out%201
      (CallFunction|AttackLeft))))

(event Custom|Drop
  (bind _currentbullet (Variables|Default|GetCurrentBullet))
  (bind _crystal_shot (Variables|/Game/Golem/BP_GolemBullet.BP_GolemBullet_C|Getcrystal_shot _currentbullet))
  (Variables|Default|SetisAttackLeft false)
  (Variables|Default|SetisAttackRight false)
  (Transformation|DetachFromActor (Variables|Default|GetCurrentBullet) "KeepWorld" "KeepWorld" "KeepWorld")
  (Physics|SetSimulatePhysics _crystal_shot true)
  (Physics|SetPhysicsLinearVelocity _crystal_shot (* (Math|Vector|GetUnitDirection(Vector) (Transformation|GetActorLocation (Variables|Default|GetCurrentBullet)) (Transformation|GetWorldLocation (Variables|Default|GetVehicle))) 5000) false "None"))

(event Custom|Attack%20Left
  (bind _returnvalue (Game|SpawnActorfromClass "/Game/Golem/BP_GolemBullet.BP_GolemBullet_C" (Math|Transform|MakeTransform (Transformation|GetWorldLocation (Variables|Default|GetLeft%20Bullet%20Spawn)) "0, 0, 0" "1.000000,1.000000,1.000000") "Undefined" "MultiplyWithRoot" 0 0))
  (bind _output_get (Variables|Default|SetCurrentBullet _returnvalue))
  (Transformation|AttachComponentToComponent _output_get (Variables|Default|GetSK_Golem_new) "hand_l_projectile" "SnapToTarget" "KeepRelative" "KeepRelative" true)
  (Utilities|FlowControl|Delay 2.0)
  (Variables|Default|SetisAttackLeft true))

(fn ConstructionScript)