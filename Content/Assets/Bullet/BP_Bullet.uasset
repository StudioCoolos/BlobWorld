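; BP_Bullet is a bullet actor that animates its scale on spawn and leaves a blob decal where it hits.
; On BeginPlay it caches the Bullet component's world scale, then a timeline multiplies that base scale as it plays.
; On component hit it spawns the decal oriented to the surface normal, sets it to fade out and self-destroy, then destroys itself.
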(event OnComponentHit(Bullet)
  (params (HitComponent :type Primitive%20Component%20Object%20Reference) (OtherActor :type Actor%20Object%20Reference) (OtherComp :type Primitive%20Component%20Object%20Reference) (NormalImpulse :type Vector :default "0, 0, 0") (Hit :type Hit%20Result%20Structure%20%28by%20ref%29))
  (bind _returnvalue (Rendering|Decal|SpawnDecalatLocation "/Game/Assets/Bullet/M_Decal_Blob.M_Decal_Blob" "100.000000,100.000000,100.000000" (.location Hit) (Math|Conversions|RotationFromXVector (.normal Hit)) 0.0))
  (Rendering|Components|Decal|SetFadeOut _returnvalue 1.0 1e+01 true)
  (Actor|DestroyActor))

(event EventBeginPlay
  (Variables|Default|SetbaseScale (Transformation|GetWorldScale (Variables|Default|GetBullet)))
  (bind _scale (Timeline|Scale_Timeline PlayFromStart)
    (:Update
      (Transformation|SetWorldScale3D (Variables|Default|GetBullet) (* _scale (Variables|Default|GetbaseScale))))))

(fn ConstructionScript)