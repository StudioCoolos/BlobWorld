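; BP_Blob is a talking blob character that plays voice lines by row name from a data table.
; While audio plays, it samples precomputed NRT loudness at the playback position to set MouthOpenFactor for lip sync.
; A request made mid-line waits out the remaining duration plus a short pause, then retries.
; DisplayBlob reveals it with a timeline-driven vertical jump, and onShoot briefly sets a shooting flag when it is silent.
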(event OnAudioPlaybackPercent(voice)
  (params (PlayingSoundWave :type Sound%20Wave%20Object%20Reference) (PlaybackPercent :type Float%20%28single-precision%29))
  (Variables|Default|SetAudioPlayBackPercent PlaybackPercent)
  (Variables|Default|SetMouthOpenFactor (Class|LoudnessNRT|GetNormalizedChannelLoudnessatTime (Variables|Default|GetActiveAudioNRT) (* PlaybackPercent (Variables|Default|GetAudioDuration)))))

(event OnAudioFinished(voice)
  (Variables|Default|SetMouthOpenFactor 0.0)
  (Variables|Default|SetisTalking false))

(event Custom|Play%20Audio
  (params (Audio%20Row%20Name :type Name))
  (Variables|Default|SetisShooting false)
  (bind _returnvalue (Utilities|GetDataTableRow "/Game/Sound_Design/Voice_Blob/Blob_Audios_DataTable.Blob_Audios_DataTable" Audio%20Row%20Name)
    (:then
      (if (Variables|Default|GetisTalking) :!label _label
        (Development|PrintString "DOUBLE PLAY" false true "(R=0.000000,G=0.660000,B=1.000000,A=1.000000)" 2e+01)
        (Utilities|FlowControl|Delay (+ (- (Variables|Default|GetAudioDuration) (* (Variables|Default|GetAudioDuration) (Variables|Default|GetAudioPlayBackPercent))) 0.5))
        (Development|PrintString "DELAY FINI" false true "(R=0.000000,G=0.660000,B=1.000000,A=1.000000)" 2e+01)
        (goto _label)
        (else
          (Variables|Default|SetActiveAudio _returnvalue)
          (Variables|Default|SetActiveAudioNRT (.Audio (Utilities|Struct|BreakBlob_Audio_Struct _returnvalue)))
          (Audio|Components|Audio|SetSound (Variables|Default|Getvoice) (Variables|/Script/AudioAnalyzer.AudioAnalyzerNRT|GetSound (.Audio (Utilities|Struct|BreakBlob_Audio_Struct _returnvalue))))
          (Variables|Default|SetAudioDuration (Variables|/Script/Engine.SoundBase|GetDuration (Variables|/Script/AudioAnalyzer.AudioAnalyzerNRT|GetSound (.Audio (Utilities|Struct|BreakBlob_Audio_Struct _returnvalue)))))
          (Audio|Components|Audio|Play (Variables|Default|Getvoice) 0.0)
          (Variables|Default|SetisTalking true))))
    (:RowNotFound
      (Development|PrintString "LE NOM DE L'AUDIO MATCH PAS LA DATABASE ENCULé " true true "(R=0.000000,G=0.660000,B=1.000000,A=1.000000)" 1e+01))))

(event Custom|DisplayBlob
  (Rendering|SetVisibility (Variables|Default|GetBlob) true true)
  (Class|AudioComponent|SetPaused (Variables|Default|Getvoice) false)
  (Variables|Default|SetisJumping true)
  (Transformation|SetRelativeLocation (Variables|Default|GetBlob) "0.000000,0.000000,1000.000000" false false)
  (bind _positionz (Timeline|Timeline PlayFromStart)
    (:Update
      (Transformation|SetRelativeLocation (Variables|Default|GetBlob) (Math|Vector|MakeVector 0.0 0.0 (* _positionz 1e+03)) false false))
    (:Finished
      (Variables|Default|SetisJumping false))))

(event Custom|onShoot
  (if (not (Variables|Default|GetisTalking))
    (Variables|Default|SetisShooting true)
    (Utilities|FlowControl|Delay 1.0)
    (Variables|Default|SetisShooting false)))

(event Custom|onShootStart)

(event EventBeginPlay)

(event Collision|EventActorBeginOverlap
  (params (OtherActor :type Actor%20Object%20Reference)))

(event EventTick
  (params (DeltaSeconds :type Float%20%28single-precision%29)))

(fn ConstructionScript)