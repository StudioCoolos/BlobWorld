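; Radio Blueprint that plays, stops and adjusts the volume of 2D music in response to the GameMode's OnRadio event, cached in the construction script.
; Play looks up a song row in DT_Radio, plays a switch sound, replaces CurrentSong and shows the row name.
; Pause stops the song and clears the text.
; Volume updates playback and briefly shows the level, using a retriggerable delay before restoring the sound's name.
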(event OnRadio(GameMode)
  (params (type :type String) (value :type String))
  (switch string type
    (:play
      (bind _returnvalue (Utilities|GetDataTableRow "/Game/Assets/Radio/DT_Radio.DT_Radio" (Utilities|String|StringToName value))
        (:then
          (Audio|PlaySound2D "/Game/Assets/Radio/Music/switch.switch" (Variables|Default|GetVolume) 1.0 0.0 0 0)
          (bind _currentsong (Variables|Default|GetCurrentSong)
            (:then
              (Audio|Components|Audio|Stop _currentsong))
            (:else
              _))
          (bind _returnvalue_2 (Audio|CreateSound2D (.src _returnvalue) (Variables|Default|GetVolume) 1.0 0.0 0))
          (bind _output_get (Variables|Default|SetCurrentSong _returnvalue_2))
          (Audio|Components|Audio|Play _output_get 0.0)
          (Rendering|Components|TextRender|SetText (Variables|Default|GetText) (Utilities|Text|ToText(String) value)))))
    (:pause
      (Audio|Components|Audio|Stop (Variables|Default|GetCurrentSong))
      (Rendering|Components|TextRender|SetText (Variables|Default|GetText) (Utilities|Text|MakeLiteralText "")))
    (:volume
      (bind _output_get_2 (Variables|Default|SetVolume (Math|Conversions|ToFloat(Integer) value)))
      (Audio|Components|Audio|SetVolumeMultiplier (Variables|Default|GetCurrentSong) _output_get_2 :!class /Script/Engine.AudioComponent)
      (Rendering|Components|TextRender|SetText (Variables|Default|GetText) (Utilities|Text|FormatText "Volume : {Volume}" (Variables|Default|GetVolume)))
      (Utilities|FlowControl|RetriggerableDelay 1.0)
      (Rendering|Components|TextRender|SetText (Variables|Default|GetText) (Utilities|Text|ToText(String) (Utilities|GetDisplayName (Variables|/Script/Engine.AudioComponent|GetSound (Variables|Default|GetCurrentSong))))))))

(event EventBeginPlay)

(event Collision|EventActorBeginOverlap
  (params (OtherActor :type Actor%20Object%20Reference)))

(event EventTick
  (params (DeltaSeconds :type Float%20%28single-precision%29)))

(fn ConstructionScript
  (bind _asgame_mode (Utilities|Casting|CastToGameMode (Game|GetGameMode)))
  (Variables|Default|SetGame%20Mode _asgame_mode))