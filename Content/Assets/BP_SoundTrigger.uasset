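; BP_SoundTrigger is a trigger volume that sends an audio event over a WebSocket when a vehicle enters it.
; On BeginPlay it caches the cast GameMode, which holds the WebSocket.
; When an actor of class BP_Vehicle or a child overlaps TriggerZone, it formats RecipientName and AudioName into a JSON-style message and sends it.
; It plays no sound itself and fires on every qualifying overlap.
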(event OnComponentBeginOverlap(TriggerZone)
  (params (OverlappedComponent :type Primitive%20Component%20Object%20Reference) (OtherActor :type Actor%20Object%20Reference) (OtherComp :type Primitive%20Component%20Object%20Reference) (OtherBodyIndex :type Integer) (bFromSweep :type Boolean) (SweepResult :type Hit%20Result%20Structure%20%28by%20ref%29))
  (if (Utilities|ClassIsChildOf (Utilities|GetClass OtherActor) "/Game/Assets/Vehicule/BP_Vehicle.BP_Vehicle_C")
    (Class|WebSocket|SendMessage (Variables|/Game/GameMode.GameMode_C|GetWebSocket (Variables|Default|GetGame%20Mode)) (Utilities|String|ToString(Text) (Utilities|Text|FormatText "`{\"event\": \"audio\", \"recipient\": \"{RecipientName}\", \"name\": \"{AudioName}\"`}" (Variables|Default|GetAudioName) (Variables|Default|GetRecipientName))))))

(event EventBeginPlay
  (bind _asgame_mode (Utilities|Casting|CastToGameMode (Game|GetGameMode)))
  (Variables|Default|SetGame%20Mode _asgame_mode))

(event Collision|EventActorBeginOverlap
  (params (OtherActor :type Actor%20Object%20Reference)))

(event EventTick
  (params (DeltaSeconds :type Float%20%28single-precision%29)))

(fn ConstructionScript)