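; Compass actor that turns to point at BP_CompassTarget actors one after another, in sorted display-name order.
; BeginPlay gathers the targets and sorts their names, then FindTarget picks the actor matching the current name and advances the index.
; Tick sets only yaw via look-at rotation, moving to the next target once the current one is invalid.
; ActorSortFunction is an empty, unfinished stub.
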(event Custom|Event_FindTarget
  (for _array_element (Variables|Default|GetCompassTargets)
    (if (Utilities|Enum|Equal(Enum) (Utilities|GetDisplayName _array_element) (Utilities|Array|Get(acopy) (Variables|Default|GetCompassTargetsNames) (Variables|Default|GetNamesIndex)))
      (Variables|Default|SetTarget _array_element)))
  (Math|Integer|IncrementInt (Variables|Default|GetNamesIndex)))

(event EventBeginPlay
  (bind _outactors (Actor|GetAllActorsOfClass "/Game/Assets/Compass/BP_CompassTarget.BP_CompassTarget_C"))
  (bind _output_get (Variables|Default|SetCompassTargets _outactors))
  (for _array_element _output_get
    (Utilities|Array|Add (Variables|Default|GetCompassTargetsNames) (Utilities|GetDisplayName _array_element)))
  (Class|KismetArrayLibrary|SortStringArray (Variables|Default|GetCompassTargetsNames))
  (CallFunction|EventFindTarget))

(event EventTick
  (params (DeltaSeconds :type Float%20%28single-precision%29))
  (bind _target (Variables|Default|GetTarget))
  (Utilities|IsValid _target
    (:Is%20Valid
      (Transformation|SetActorRotation (Math|Rotator|MakeRotator 0.0 0.0 (.yaw (Math|Rotator|FindLookatRotation (Transformation|GetActorLocation) (Transformation|GetActorLocation _target)))) true))
    (:Is%20Not%20Valid
      (CallFunction|EventFindTarget))))

(fn ConstructionScript)

(fn ActorSortFunction
  (params (Actor%20A :type Actor%20Object%20Reference) (Actor%20B :type Actor%20Object%20Reference)))